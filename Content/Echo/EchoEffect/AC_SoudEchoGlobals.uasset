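; Global sound echo component that shows sounds as expanding, fading waves through a post-process material.
; On BeginPlay it puts a dynamic MI_EchoPostProcess on the "Global"-tagged PostProcessVolume and fills a pool of wave indices.
; ShowSound claims an index; Tick grows each radius, fades alpha, writes both plus location to MPC_SoundEchos and recycles finished indices.
; Render-target data-texture functions and the update throttle are never called here.
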(event `self.ReceiveBeginPlay`
  (`self.Setup`))

(event `self.ReceiveTick`
  (params (DeltaSeconds :type "Float (single-precision)"))
  (`self.UpdateWavesData`))

(fn `AddSoundEchoEffectDMI`
  (locals (Result :type "Array of PostProcessVolume Object Reference") (GlobalPostProcessSettings :type "PostProcessSettings Structure") (PostProcessMaterials :type "WeightedBlendables Structure"))
  (`|ExecutionSequence`
    (:`then_0`
      (bind _outactors (`GameplayStatics.GetAllActorsOfClassWithTag` "/Script/Engine.PostProcessVolume" "Global"))
      (bind _output_get (set `local.Result` _outactors))
      (if (`KismetArrayLibrary.Array_IsEmpty` _output_get)
        (`KismetSystemLibrary.PrintString` "Error: Could not find actor of PostProcessVolume class in level with tag \"Global\"" true true (struct :`R` 1.0 :`G` 0.03618 :`A` 1.0) 5.0)
        (else
          (bind _returnvalue (`KismetMaterialLibrary.CreateDynamicMaterialInstance` "/Game/Echo/EchoEffect/Materials/MI_EchoPostProcess.MI_EchoPostProcess" "EchoSoundVisualEffect"))
          (set `self.EchoDynamicMaterialInstance` _returnvalue)
          (bind _output_get_2 (set `self.GlobalPostProcessVolume` (`|GetArrayItem` (`local.Result`))))
          (set `local.GlobalPostProcessSettings` (`PostProcessVolume.Settings` _output_get_2))
          (set `local.PostProcessMaterials` (`.WeightedBlendables` (break `PostProcessSettings` (`local.GlobalPostProcessSettings`))))
          (setmembers `WeightedBlendables` :`StructRef` (`local.PostProcessMaterials`) :`Array` (`|MakeArray` (make `WeightedBlendable` 1.0 (`self.EchoDynamicMaterialInstance`))))
          (setmembers `PostProcessSettings` :`StructRef` (`local.GlobalPostProcessSettings`) :`WeightedBlendables` (`local.PostProcessMaterials`))
          (set `PostProcessVolume.Settings` (`local.GlobalPostProcessSettings`) (`self.GlobalPostProcessVolume`)))))))

(fn `ClearTarget`
  (locals (PixelsXCount :type Integer) (Canvas :type "Canvas Object Reference") (Context :type "DrawToRenderTargetContext Structure"))
  (`|ExecutionSequence`
    (:`then_0`
      (bind (_canvas _size _context) (`KismetRenderingLibrary.BeginDrawCanvasToRenderTarget` (`self.RenderTarget`)))
      (set `local.Canvas` _canvas)
      (set `local.Context` _context)
      (set `local.PixelsXCount` (`KismetMathLibrary.FTrunc` (`KismetMathLibrary.BreakVector2D` _size))))
    (:`then_1`
      (`Canvas.K2_DrawBox` (`local.Canvas`) (`KismetMathLibrary.MakeVector2D` 0.0) (`KismetMathLibrary.MakeVector2D` 1.0 1.0) 1.0 (make `LinearColor` 0.0)))
    (:`then_2`
      (`KismetRenderingLibrary.EndDrawCanvasToRenderTarget` (`local.Context`))
      (`MaterialInstanceDynamic.SetTextureParameterValue` (`self.EchoDynamicMaterialInstance`) (`self.EchoDataParamName`) (`self.RenderTarget`)))))

(fn `CreateRenderTarget`
  (bind _returnvalue (`KismetRenderingLibrary.CreateRenderTarget2D` (* (`self.MaxSoundEchoEffects`) 2) 1 "RTF_RGBA32f" (make `LinearColor` 0.0) false true))
  (set `self.RenderTarget` _returnvalue)
  (`|ExecutionSequence`
    (:`then_0`
      (set `TextureRenderTarget2D.AddressX` "TA_Wrap" (`self.RenderTarget`))
      (set `TextureRenderTarget2D.AddressY` "TA_Wrap" (`self.RenderTarget`))
      (set `Texture.MipGenSettings` "TMGS_NoMipmaps" (`self.RenderTarget`)))
    (:`then_1`
      (set `Texture.Filter` "TF_Nearest" (`self.RenderTarget`))
      (set `Texture.CompressionSettings` "TC_EditorIcon" (`self.RenderTarget`))
      (set `Texture.LODGroup` "TEXTUREGROUP_Pixels2D" (`self.RenderTarget`)))))

(fn `SetMaterialDataAtIndex`
  (params (Canvas :type "Canvas Object Reference") (EchoEffect :type "/Game/Echo/EchoEffect/F_SoundEcho Structure") (Index :type Integer) (SizeX :type "Float (double-precision)"))
  (locals (EchoEffect :type "/Game/Echo/EchoEffect/F_SoundEcho Structure") (Index :type Integer) (PixelSize :type "Float (double-precision)"))
  (bind ((`Location_2_491E519C44DBF337A289488D0D16E2F1` _location) (`Alpha_10_553F933B456DEEEA68C8A3A4515A637E` _alpha)) (break `/Game/Echo/EchoEffect/F_SoundEcho` (`local.EchoEffect`)))
  (set `local.PixelSize` (/ 1.0 (`local.SizeX`)))
  (`Canvas.K2_DrawBox` (`local.Canvas`) (`KismetMathLibrary.MakeVector2D` (`KismetMathLibrary.SafeDivide` (`KismetMathLibrary.Conv_IntToDouble` (`local.Index`)) (`local.SizeX`))) (`KismetMathLibrary.MakeVector2D` (`local.PixelSize`) 1.0) 1.0 (make `LinearColor` (.x _location) (.y _location) (.z _location) _alpha)))

(fn `Setup`
  (`self.AddSoundEchoEffectDMI`)
  (for _index (range (`self.MaxSoundEchoEffects`))
    (`KismetArrayLibrary.Array_Add` (`self.AvailableWavesIndexes`) _index)))

(fn `ShouldUpdateEcho`
  (returns (ShouldUpdate :type Boolean))
  (bind _output_get (set `self.UpdateTimeCounterSeconds` (+ (`GameplayStatics.GetWorldDeltaSeconds`) (`self.UpdateTimeCounterSeconds`))))
  (if (>= _output_get (`self.UpdateTimeStep`))
    (set `self.UpdateTimeCounterSeconds` (- (`self.UpdateTimeCounterSeconds`) (`self.UpdateTimeStep`)))
    (return true)
    (else
      (return false))))

(fn `ShowSound`
  (params (Location :type "Vector Structure") (Strength :type "Float (double-precision)"))
  (if (`KismetArrayLibrary.Array_IsNotEmpty` (`self.AvailableWavesIndexes`))
    (`KismetArrayLibrary.Array_Add` (`self.Echos`) (make `/Game/Echo/EchoEffect/F_SoundEcho` Location Strength 0.0 1.0 (`|GetArrayItem` (`self.AvailableWavesIndexes`))))
    (`KismetArrayLibrary.Array_Remove` (`self.AvailableWavesIndexes`))
    (`KismetSystemLibrary.PrintString` (`KismetTextLibrary.Conv_TextToString` (`|FormatText` "AvailableIndexes: {i}" (`KismetArrayLibrary.Array_Length` (`self.AvailableWavesIndexes`)))) true false (struct :`R` 1.0 :`G` 0.298039 :`A` 1.0) 9999.0 "AvailableIndexes")
    (else
      (`KismetSystemLibrary.PrintString` "No mask index left" true true (struct :`R` 1.0 :`A` 1.0) 5.0))))

(fn `UpdateRenderTarget`
  (locals (Canvas :type "Canvas Object Reference") (Context :type "DrawToRenderTargetContext Structure") (EchoEffect :type "/Game/Echo/EchoEffect/F_SoundEcho Structure") (Size :type "Vector2D Structure") (Index :type Integer))
  (bind _size_x (`KismetMathLibrary.BreakVector2D` (`local.Size`)))
  (bind (_location _maxradius _radius _alpha) (break `/Game/Echo/EchoEffect/F_SoundEcho` (`local.EchoEffect`)))
  (bind _returnvalue (+ (`local.Index`) 1))
  (`|ExecutionSequence`
    (:`then_0`
      (bind (_canvas _size _context) (`KismetRenderingLibrary.BeginDrawCanvasToRenderTarget` (`self.RenderTarget`)))
      (set `local.Canvas` _canvas)
      (set `local.Size` _size)
      (set `local.Context` _context)
      (`KismetSystemLibrary.PrintString` (`KismetTextLibrary.Conv_TextToString` (`|FormatText` "Texture Size: {v}" (`KismetStringLibrary.Conv_Vector2dToString` (`local.Size`)))) true true (struct :`G` 0.66 :`B` 1.0 :`A` 1.0) 2.0 "TextureSize"))
    (:`then_1`
      (for (_array_element _array_index) (`self.Echos`)
        (bind _output_get (set `local.EchoEffect` _array_element))
        (bind _output_get_2 (set `local.Index` _array_index))
        (`self.SetMaterialDataAtIndex` (`local.Canvas`) _output_get _output_get_2 _size_x)))
    (:`then_2`
      (`KismetRenderingLibrary.EndDrawCanvasToRenderTarget` (`local.Context`))
      (`MaterialInstanceDynamic.SetTextureParameterValue` (`self.EchoDynamicMaterialInstance`) (`self.EchoDataParamName`) (`self.RenderTarget`)))
    (:`then_3`
      (for (_array_element_2 _array_index_2) (`self.Echos`)
        (set `local.Index` _array_index_2)
        (set `local.EchoEffect` _array_element_2)
        (`KismetSystemLibrary.PrintString` (`KismetTextLibrary.Conv_TextToString` (`|FormatText` "Updated pixel: \n- location: {l} \n- Max Rad: {x} \n- Radius: {r} \n- Alpha: {a}" (`KismetStringLibrary.Conv_VectorToString` _location) _maxradius _radius _alpha)) true true (struct :`G` 0.66 :`B` 1.0 :`A` 1.0) 3.0 (`KismetStringLibrary.Conv_StringToName` (`KismetStringLibrary.Conv_IntToString` (`local.Index`))))
        (`|ExecutionSequence`
          (:`then_0`
            (bind _returnvalue_2 (`KismetRenderingLibrary.ReadRenderTargetPixel` (`self.RenderTarget`) (`local.Index`)))
            (bind _result (`|FormatText` "Pixel {i}: {p1}" (`local.Index`) (`KismetStringLibrary.Conv_ColorToString` (`KismetMathLibrary.Conv_ColorToLinearColor` _returnvalue_2))))
            (`KismetSystemLibrary.PrintString` (`KismetTextLibrary.Conv_TextToString` _result) true true (struct :`G` 0.66 :`B` 1.0 :`A` 1.0) 3.0 (`KismetStringLibrary.Conv_StringToName` (`KismetTextLibrary.Conv_TextToString` _result))))
          (:`then_1`
            (bind _returnvalue_3 (`KismetRenderingLibrary.ReadRenderTargetPixel` (`self.RenderTarget`) _returnvalue))
            (bind _result_2 (`|FormatText` "Pixel {i}: {p1}" _returnvalue (`KismetStringLibrary.Conv_ColorToString` (`KismetMathLibrary.Conv_ColorToLinearColor` _returnvalue_3))))
            (`KismetSystemLibrary.PrintString` (`KismetTextLibrary.Conv_TextToString` _result_2) true true (struct :`G` 0.66 :`B` 1.0 :`A` 1.0) 3.0 (`KismetStringLibrary.Conv_StringToName` (`KismetTextLibrary.Conv_TextToString` _result_2)))))))))

(fn `UpdateWavesData`
  (locals (DeleteList :type "Array of Integer") (EchoEffect :type "/Game/Echo/EchoEffect/F_SoundEcho Structure") (LoopIndex :type Integer) (ParamIndex :type Integer))
  (bind ((`MaxRadius_5_917967744FEBD82C398A2C9FA3CBF853` _maxradius) (`Radius_7_E1571D5D44BD2E8F4D881CA665BE3A39` _radius)) (break `/Game/Echo/EchoEffect/F_SoundEcho` (`local.EchoEffect`)))
  (bind ((`MaxRadius_5_917967744FEBD82C398A2C9FA3CBF853` _maxradius_2) (`Radius_7_E1571D5D44BD2E8F4D881CA665BE3A39` _radius_2)) (break `/Game/Echo/EchoEffect/F_SoundEcho` (`local.EchoEffect`)))
  (bind (_location _maxradius_3 _radius_3 _alpha) (break `/Game/Echo/EchoEffect/F_SoundEcho` (`local.EchoEffect`)))
  (bind ((`Location_2_491E519C44DBF337A289488D0D16E2F1` _location_2) (`Alpha_10_553F933B456DEEEA68C8A3A4515A637E` _alpha_2)) (break `/Game/Echo/EchoEffect/F_SoundEcho` (`local.EchoEffect`)))
  (`KismetSystemLibrary.PrintString` (`KismetTextLibrary.Conv_TextToString` (`|FormatText` "Sound Waves Count: {c}" (`KismetArrayLibrary.Array_Length` (`self.Echos`)))) true true (struct :`G` 1.0 :`B` 0.003935 :`A` 1.0) 2.0 "SoundWavesCount")
  (if (`KismetArrayLibrary.Array_IsNotEmpty` (`self.Echos`))
    (`|ExecutionSequence`
      (:`then_0`
        (for (_array_element _array_index) (`self.Echos`)
          (bind _output_get (set `local.EchoEffect` _array_element))
          (set `local.LoopIndex` _array_index)
          (set `local.ParamIndex` (`.WaveIndex_14_494E3EFC44E6E360DFF6CF8680C8A2F1` (break `/Game/Echo/EchoEffect/F_SoundEcho` _output_get)))
          (`|ExecutionSequence`
            (:`then_0`
              (if (< _radius_2 _maxradius_2)
                (bind _structout (setmembers `/Game/Echo/EchoEffect/F_SoundEcho` :`StructRef` (`local.EchoEffect`) :`Radius` (`KismetMathLibrary.FClamp` (+ _radius (* (`self.DefaultWaveSpeed`) (`GameplayStatics.GetWorldDeltaSeconds`))) 0.0 _maxradius)))
                (`KismetArrayLibrary.Array_Set` (`self.Echos`) (`local.LoopIndex`) _structout)
                (elif (> (`.Alpha_10_553F933B456DEEEA68C8A3A4515A637E` (break `/Game/Echo/EchoEffect/F_SoundEcho` (`local.EchoEffect`))) 0.0)
                  (bind _structout_2 (setmembers `/Game/Echo/EchoEffect/F_SoundEcho` :`StructRef` (`local.EchoEffect`) :`Alpha` (`KismetMathLibrary.FClamp` (- (`.Alpha_10_553F933B456DEEEA68C8A3A4515A637E` (break `/Game/Echo/EchoEffect/F_SoundEcho` (`local.EchoEffect`))) (* (`self.VisualsFadeRate`) (`GameplayStatics.GetWorldDeltaSeconds`))))))
                  (`KismetArrayLibrary.Array_Set` (`self.Echos`) (`local.LoopIndex`) _structout_2)
                  (else
                    (`KismetArrayLibrary.Array_Add` (`local.DeleteList`) (`local.LoopIndex`))
                    (`KismetArrayLibrary.Array_Insert` (`self.AvailableWavesIndexes`) (`local.ParamIndex`))
                    (`KismetSystemLibrary.PrintString` (`KismetTextLibrary.Conv_TextToString` (`|FormatText` "AvailableIndexes: {i}" (`KismetArrayLibrary.Array_Length` (`self.AvailableWavesIndexes`)))) true false (struct :`R` 1.0 :`G` 0.298039 :`A` 1.0) 9999.0 "AvailableIndexes")))))
            (:`then_1`
              (`KismetMaterialLibrary.SetVectorParameterValue` "/Game/Echo/EchoEffect/Materials/MPC_SoundEchos.MPC_SoundEchos" (`KismetStringLibrary.Conv_StringToName` (`KismetStringLibrary.Concat_StrStr` (`KismetStringLibrary.Conv_NameToString` "Location") (`KismetStringLibrary.Conv_IntToString` (`local.ParamIndex`)))) (make `LinearColor` (.x _location_2) (.y _location_2) (.z _location_2) _alpha_2))
              (`KismetMaterialLibrary.SetVectorParameterValue` "/Game/Echo/EchoEffect/Materials/MPC_SoundEchos.MPC_SoundEchos" (`KismetStringLibrary.Conv_StringToName` (`KismetStringLibrary.Concat_StrStr` (`KismetStringLibrary.Conv_NameToString` "Size") (`KismetStringLibrary.Conv_IntToString` (`local.ParamIndex`)))) (make `LinearColor` (`.Radius_7_E1571D5D44BD2E8F4D881CA665BE3A39` (break `/Game/Echo/EchoEffect/F_SoundEcho` (`local.EchoEffect`))))))
            (:`then_2`
              (`KismetSystemLibrary.PrintString` (`KismetTextLibrary.Conv_TextToString` (`|FormatText` "Updated pixel: \n- index: {i} \n- location: {l} \n- Max Rad: {x} \n- Radius: {r} \n- Alpha: {a} \nParams set: \n{1} \n{2}" (`local.ParamIndex`) (`KismetStringLibrary.Conv_VectorToString` _location) _maxradius_3 _radius_3 _alpha (`KismetStringLibrary.Conv_StringToName` (`KismetStringLibrary.Concat_StrStr` (`KismetStringLibrary.Conv_NameToString` "Location") (`KismetStringLibrary.Conv_IntToString` (`local.ParamIndex`)))) (`KismetStringLibrary.Conv_StringToName` (`KismetStringLibrary.Concat_StrStr` (`KismetStringLibrary.Conv_NameToString` "Size") (`KismetStringLibrary.Conv_IntToString` (`local.ParamIndex`)))))) true true (struct :`G` 0.66 :`B` 1.0 :`A` 1.0) 3.0 (`KismetStringLibrary.Conv_StringToName` (`KismetStringLibrary.Conv_IntToString` (`local.ParamIndex`))))))))
      (:`then_1`
        (for _array_element_2 (`local.DeleteList`)
          (`KismetArrayLibrary.Array_Remove` (`self.Echos`) _array_element_2))))))